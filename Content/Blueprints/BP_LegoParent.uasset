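; Base Lego piece actor that becomes a random physics-simulated brick on BeginPlay.
; It picks a random row from DT_LegoParts for its mesh, then a color from that part's allowed set, or any color if empty, via the DT_Colors map.
; SetUnlit swaps in an unlit material and line-traces from a given point, showing the piece's color when it is the first hit and black otherwise.
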(event EventBeginPlay
  (CallFunction|InitializeLego))

(fn ConstructionScript)

(fn InitializeLego
  (CallFunction|SetupBaseValues)
  (CallFunction|SetMeshandColor)
  (Physics|SetSimulatePhysics (Variables|Default|GetMesh) true))

(fn SetupBaseValues
  (bind _outrownames (DataTable|GetDataTableRowNames "/Game/DT_LegoParts.DT_LegoParts"))
  (bind _output_get (Variables|Default|SetCurrentLegoName (.OutItem (Utilities|Array|Random _outrownames))))
  (bind _returnvalue (Utilities|GetDataTableRow "/Game/DT_LegoParts.DT_LegoParts" _output_get)
    (:then
      (Variables|Default|SetCurrentLegoStruct _returnvalue))))

(fn SetMeshandColor
  (Components|StaticMesh|SetStaticMesh (Variables|Default|GetMesh) (Utilities|Struct|BreakS_Lego (Variables|Default|GetCurrentLegoStruct)))
  (bind _returnvalue (CallFunction|GetRandomColor))
  (Variables|Default|SetMeshColor _returnvalue)
  (bind _returnvalue_2 (Rendering|Material|CreateDynamicMaterialInstance (Variables|Default|GetMesh) 0 (Variables|Default|GetMaterial) "" :!class /Script/Engine.PrimitiveComponent))
  (Rendering|Material|SetVectorParameterValue _returnvalue_2 "Color" _returnvalue :!class /Script/Engine.MaterialInstanceDynamic))

(fn GetRandomColor
  (bind _returnvalue (Utilities|GetDataTableRow "/Game/DT_Colors.DT_Colors" "Colors")
    (:then
      (LocalVariables|SetColorsMap (Utilities|Struct|BreakS_Colors _returnvalue))
      (if (Utilities|Set|IsEmpty (Utilities|Struct|BreakS_Lego (Variables|Default|GetCurrentLegoStruct))) ; If lego doesnt have colors then get random color from all colors
        (return (Math|Conversions|ToLinearColor(Color) (.Value (Utilities|Map|Find (LocalVariables|GetColorsMap) (Utilities|Enum|ByteToEnumColorsEnum (Math|Conversions|ToByte(Integer) (Math|Random|RandomIntegerinRange 0 (Math|Conversions|ToInteger(Byte) (Math|Byte|MakeLiteralByte (Utilities|Enum|LiteralenumColorsEnum "NewEnumerator32"))))))))))
        (else
          (bind _result (Utilities|Set|ToArray (Utilities|Struct|BreakS_Lego (Variables|Default|GetCurrentLegoStruct))))
          (return (Math|Conversions|ToLinearColor(Color) (.Value (Utilities|Map|Find (LocalVariables|GetColorsMap) (.OutItem (Utilities|Array|Random _result)))))))))))

(fn SetUnlit
  (params (Start :type Vector))
  (bind _returnvalue (Rendering|Material|CreateDynamicMaterialInstance (Variables|Default|GetMesh) 0 "/Game/LEGOs/Materials/UnlitLegoMaterial.UnlitLegoMaterial" "" :!class /Script/Engine.PrimitiveComponent))
  (LocalVariables|SetDynamicMaterial _returnvalue)
  (bind (_outhit _returnvalue_2) (Collision|LineTraceForObjects Start (+ (* (Math|Vector|Normalize (- (Transformation|GetWorldLocation (Variables|Default|GetMesh)) Start)) 10) (Transformation|GetWorldLocation (Variables|Default|GetMesh))) (Utilities|Array|MakeArray "ObjectTypeQuery4") false 0 "None" false "(R=1.000000,G=0.000000,B=0.000000,A=1.000000)" "(R=0.000000,G=1.000000,B=0.000000,A=1.000000)" 1.0))
  (if _returnvalue_2
    (if (== (.HitActor (Collision|BreakHitResult _outhit)) self)
      (Rendering|Material|SetVectorParameterValue (LocalVariables|GetDynamicMaterial) "Color" (Variables|Default|GetMeshColor) :!class /Script/Engine.MaterialInstanceDynamic)
      (else
        (Rendering|Material|SetVectorParameterValue :self (LocalVariables|GetDynamicMaterial) :ParameterName "Color" :!class /Script/Engine.MaterialInstanceDynamic :!label _label)))
    (else
      (goto _label))))