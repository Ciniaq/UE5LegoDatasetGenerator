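; Screenshot manager that automatically captures paired original and mask-style images of randomly floored Lego scenes, apparently as a dataset generator.
; Once all spawners report done, it culls neighboring pieces, briefly simulates physics, then freezes them.
; From each camera it takes a high-res lit shot, then an unlit shot with black floors via show flags and material swaps.
; After the last camera it respawns the scene, quitting past a photo limit.
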(event Custom|EventMakeScreenshots
  (bind _returnvalue (Math|DateTime|Now))
  (bind (_year _month _day _hour _minute _second) (Math|DateTime|BreakDateTime _returnvalue))
  (Variables|Default|SetCurrentScreensName (Utilities|Text|FormatText "{day}-{hour}{minute}{second}" _day _hour _minute _second))
  (Utilities|FlowControl|Delay 2.0)
  (CallFunction|TakeCommandScreenshot (Utilities|Text|FormatText "{date_time}_original.png" (Variables|Default|GetCurrentScreensName)) true)
  (Utilities|FlowControl|Delay 1.0)
  (CallFunction|SetSceneUnlit)
  (Utilities|FlowControl|Delay 1.0)
  (CallFunction|TakeCommandScreenshot (Utilities|Text|FormatText "{date_time}_masked.png" (Variables|Default|GetCurrentScreensName)) true)
  (Math|Integer|IncrementInt (Variables|Default|GetPhotosDone)
    (:%20%20
      (Utilities|FlowControl|Delay 1.0)
      (CallFunction|SetupNextCamera)
      (if (> (Variables|Default|GetPhotosDone) 2100)
        (Game|QuitGame 0 "Quit" false)))))

(event Custom|RefreshPhysicsStartMakingScreenshots
  (for _array_element (Variables|Default|GetSpawners)
    (Default|LegosSetSimulatePhysics _array_element true))
  (Utilities|FlowControl|Delay 2.0)
  (for _array_element_2 (Variables|Default|GetSpawners)
    (Default|LegosSetSimulatePhysics _array_element_2 false))
  (CallFunction|EventMakeScreenshots))

(event Custom|EventKillNeighbours
  (bind _arrayindex (Utilities|LoopwithExec 0 (- (Utilities|Array|Length (Variables|Default|GetSpawners)) 1) :!label _label)
    (:LoopBody
      (Default|KillNeighborhoodSiblings (Utilities|Array|Get(acopy) (Variables|Default|GetSpawners) _arrayindex))
      (goto _label NextBody))
    (:Completed
      (bind _arrayindex_2 (Utilities|LoopwithExec 0 (- (Utilities|Array|Length (Variables|Default|GetSpawners)) 1) :!label _label_2)
        (:LoopBody
          (Default|LegosSetSimulatePhysics (Utilities|Array|Get(acopy) (Variables|Default|GetSpawners) _arrayindex_2) true)
          (goto _label_2 NextBody))
        (:Completed
          (Utilities|FlowControl|Delay 2.0)
          (bind _arrayindex_3 (Utilities|LoopwithExec 0 (- (Utilities|Array|Length (Variables|Default|GetSpawners)) 1) :!label _label_3)
            (:LoopBody
              (Default|KillNeighborhoodSiblings (Utilities|Array|Get(acopy) (Variables|Default|GetSpawners) _arrayindex_3))
              (goto _label_3 NextBody))
            (:Completed
              (CallFunction|RefreshPhysicsStartMakingScreenshots))))))))

(event EventBeginPlay
  (CallFunction|SetRandomFloorMaterial)
  (CallFunction|SetCurrentCamera)
  (Development|ExecuteConsoleCommand "ShowFlag.Lighting 1" 0)
  (Development|ExecuteConsoleCommand "ShowFlag.PostProcessing 1" 0)
  (for _array_element (Variables|Default|GetSpawners)
    (Default|EventSpawnLegos _array_element)))

(fn ConstructionScript
  (Variables|Default|SetSpawnersDone 0)
  (for _array_element (Variables|Default|GetSpawners)
    (Variables|/Game/Blueprints/BP_LegoSpawner.BP_LegoSpawner_C|SetParent _array_element self)))

(fn NotifySpawningDone
  (bind _result (Math|Integer|IncrementInt (Variables|Default|GetSpawnersDone))
    (:%20%20
      (if (== _result (Utilities|Array|Length (Variables|Default|GetSpawners)))
        (CallFunction|EventKillNeighbours)))))

(fn RestartScene
  (Development|ExecuteConsoleCommand "ShowFlag.Lighting 1" 0)
  (Development|ExecuteConsoleCommand "ShowFlag.PostProcessing 1" 0)
  (CallFunction|SetCurrentCamera)
  (Variables|Default|SetSpawnersDone 0)
  (for _array_element (Variables|Default|GetSpawners)
    (Default|ClearSpawnedLegos _array_element))
  (for _array_element_2 (Variables|Default|GetSpawners)
    (Default|EventSpawnLegos _array_element_2))
  (CallFunction|SetRandomFloorMaterial))

(fn SetSceneUnlit
  (Development|ExecuteConsoleCommand "ShowFlag.Lighting 0" 0)
  (Development|ExecuteConsoleCommand "ShowFlag.PostProcessing 0" 0)
  (for _array_element (Variables|Default|GetSpawners)
    (Default|SetUnlit _array_element (Transformation|GetWorldLocation (Variables|/Script/Engine.CameraActor|GetSceneComponent (CallFunction|GetCurrentCamera)))))
  (for _array_element_2 (Variables|Default|GetFloors)
    (Rendering|Material|SetMaterial (Variables|/Script/Engine.StaticMeshActor|GetStaticMeshComponent _array_element_2) 0 "/Engine/EngineDebugMaterials/BlackUnlitMaterial.BlackUnlitMaterial")))

(fn SetCurrentCamera
  (params (CameraIndex :type Integer))
  (Variables|Default|SetCurrentCameraIndex CameraIndex)
  (Game|Player|SetViewTargetwithBlend (Game|GetPlayerController 0) (CallFunction|GetCurrentCamera) 0.0 "VTBlend_Linear" 0.0 false))

(fn GetCurrentCamera
  (return (Utilities|Array|Get(acopy) (Variables|Default|GetMainCamera) (Variables|Default|GetCurrentCameraIndex))))

(fn SetupNextCamera
  (if (< (+ (Variables|Default|GetCurrentCameraIndex) 1) (Utilities|Array|Length (Variables|Default|GetMainCamera)))
    (CallFunction|SetCurrentCamera (+ (Variables|Default|GetCurrentCameraIndex) 1))
    (CallFunction|ResetSceneMaterials)
    (CallFunction|EventMakeScreenshots)
    (else
      (CallFunction|RestartScene))))

(fn ResetSceneMaterials
  (Development|ExecuteConsoleCommand "ShowFlag.Lighting 1" 0)
  (Development|ExecuteConsoleCommand "ShowFlag.PostProcessing 1" 0)
  (for _array_element (Variables|Default|GetSpawners)
    (Default|ResetMaterials _array_element))
  (CallFunction|SetRandomFloorMaterial))

(fn SetRandomFloorMaterial
  (LocalVariables|SetFloorMaterial (.OutItem (Utilities|Array|Random (Variables|Default|GetFloorMaterials))))
  (for _array_element (Variables|Default|GetFloors)
    (Rendering|Material|SetMaterial (Variables|/Script/Engine.StaticMeshActor|GetStaticMeshComponent _array_element) 0 (LocalVariables|GetFloorMaterial))))

(fn TakeCommandScreenshot
  (params (filename :type Text) (bCaptureHDR :type Boolean))
  (Development|ExecuteConsoleCommand (Utilities|String|ToString(Text) (Utilities|Text|FormatText "HighResShot {width}x{height} filename={filename} bCaptureHDR {bCaptureHDR}" (Utilities|Text|MakeLiteralText "1920") (Utilities|Text|MakeLiteralText "1080") filename (select bCaptureHDR (Utilities|Text|MakeLiteralText "1") (Utilities|Text|MakeLiteralText "0")))) (Game|GetPlayerController 0)))